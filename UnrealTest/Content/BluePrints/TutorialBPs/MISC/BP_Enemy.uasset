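; BP_Enemy is an enemy that walks along an array of waypoints and is destroyed when its life runs out.
; Tick checks distance to the current destination, using AI MoveTo to advance when close or head to the first waypoint while the index is zero.
; Hit sets the WB_LifeBar widget's percent before decrementing Life, so the bar lags one hit.
; LocateObjective caches the first BP_Obj but is not called here.
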(event `self.ReceiveBeginPlay`
  (set `self.MaxLife` (`self.Life`)))

(event `MoveToNextWaypoint`
  (bind _output (`self.Get Next Waypoint`))
  (bind _output_get (set `self.Destination` (`self.K2_GetActorLocation` _output)))
  (`|AIMoveTo` self _output_get null))

(event `self.ReceiveTick`
  (params (DeltaSeconds :type "Float (single-precision)"))
  (bind _returnvalue (`KismetMathLibrary.Vector_Distance` (`self.Destination`) (`self.K2_GetActorLocation`)))
  (set `self.DistanceTo` _returnvalue)
  (if (<= _returnvalue 100.0)
    (`self.MoveToNextWaypoint`)
    (elif (== (`self.WaypointIndex`) 0)
      (bind _output_get (set `self.Destination` (`self.K2_GetActorLocation` (`|GetArrayItem` (`self.Waypoints`)))))
      (`|AIMoveTo` self _output_get null))))

(event `self.ReceiveHit`
  (params (MyComp :type "PrimitiveComponent Object Reference") (Other :type "Actor Object Reference") (OtherComp :type "PrimitiveComponent Object Reference") (bSelfMoved :type Boolean) (HitLocation :type "Vector Structure") (HitNormal :type "Vector Structure") (NormalImpulse :type "Vector Structure") (Hit :type "HitResult Structure (by ref)"))
  (bind _life (`self.Life`))
  (bind _aswb_life_bar (cast `/Game/UI/WB_LifeBar` (`WidgetComponent.GetWidget` (`self.LifeBarWidget`))))
  (`ProgressBar.SetPercent` (`/Game/UI/WB_LifeBar.LifeBar` _aswb_life_bar) (/ (`self.Life`) (`self.MaxLife`)))
  (`/Engine/EditorBlueprintResources/StandardMacros.DecrementFloat` _life
    (:`  `
      (if (<= _life 0.0)
        (`self.K2_DestroyActor`)))))

(fn `Get Next Waypoint`
  (returns (Output :type "Actor Object Reference"))
  (bind _result (`/Engine/EditorBlueprintResources/StandardMacros.IncrementInt` (`self.WaypointIndex`))
    (:`  `
      (return (`|GetArrayItem` (`self.Waypoints`) _result)))))

(fn `LocateObjective`
  (bind _outactors (`GameplayStatics.GetAllActorsOfClass` "/Game/BluePrints/TutorialBPs/MISC/BP_Obj.BP_Obj_C"))
  (set `self.Obj` (`|GetArrayItem` _outactors)))

(fn `UserConstructionScript`)