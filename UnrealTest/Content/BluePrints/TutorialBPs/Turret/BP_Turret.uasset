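; Automated turret that tracks pawns tagged "Enemy" and shoots first-person projectiles at them.
; PawnSensing records the target's location, and a retriggerable delay clears the spotted flag when sightings stop.
; Tick interpolates the mesh toward that location and, when the angle between current and next interpolated rotation is small enough, fires through a rate-limiting Delay.
; FireGun alternates left and right barrel sockets, setting each projectile's speed after spawn.
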(event `self.ReceiveBeginPlay`
  ;[0.5368 0.6751 1] OnStart Variable Setup
  (set `PawnSensingComponent.SightRadius` (`self.Detection Radius`) (`self.PawnSensing`)))

(event `self.PawnSensing.OnSeePawn`
  (params (Pawn :type "Pawn Object Reference"))
  ;[1 1 1] Player Detection
  (set `self.Pawn` Pawn)
  (`|ExecutionSequence`
    (:`then_0`
      (if (`self.ActorHasTag` Pawn "Enemy")
        (set `self.PlayerSpotted` true)
        (set `self.Target Location` (`self.K2_GetActorLocation` Pawn))))
    (:`then_1`
      (`KismetSystemLibrary.RetriggerableDelay` 0.2)
      (set `self.PlayerSpotted` false))))

(event `self.ReceiveTick`
  (params (DeltaSeconds :type "Float (single-precision)"))
  (bind _returnvalue (`KismetMathLibrary.RInterpTo` (`SceneComponent.RelativeRotation` (`self.StaticMesh`)) (`KismetMathLibrary.FindLookAtRotation` (`self.K2_GetActorLocation`) (`self.Target Location`)) (`self.Delta Seconds`) (`self.RotateSpeed`)))
  (set `self.Delta Seconds` DeltaSeconds)
  (if (`self.PlayerSpotted`)
    (`SceneComponent.K2_SetRelativeRotation` (`self.StaticMesh`) _returnvalue false false)
    (bind _angle (`self.AngleTurretToPlayer` (`KismetMathLibrary.Conv_RotatorToVector` (`SceneComponent.RelativeRotation` (`self.StaticMesh`))) (`KismetMathLibrary.Conv_RotatorToVector` _returnvalue)))
    (if (<= _angle (`self.AngleToFire`))
      (`KismetSystemLibrary.Delay` (`self.RateOfFire`))
      (`self.FireGun`))))

(fn `AngleTurretToPlayer`
  (params (TurretToPlayerVector :type "Vector Structure") (CurrentTurretVector :type "Vector Structure"))
  (returns (Angle :type "Float (double-precision)"))
  (bind _returnvalue (`KismetMathLibrary.Normal` TurretToPlayerVector))
  (bind _returnvalue_2 (`KismetMathLibrary.Normal` CurrentTurretVector))
  (return (`KismetMathLibrary.DegAcos` (/ (`KismetMathLibrary.Dot_VectorVector` _returnvalue _returnvalue_2) (* (`KismetMathLibrary.VSize` _returnvalue) (`KismetMathLibrary.VSize` _returnvalue_2))))))

(fn `FireGun`
  (if (`self.LeftRailgun`)
    (bind _returnvalue (`|SpawnActorFromClass` "/Game/FirstPerson/Blueprints/BP_FirstPersonProjectile.BP_FirstPersonProjectile_C" (`SceneComponent.GetSocketTransform` (`self.StaticMesh`) "LeftBarrel" "RTS_World") "Undefined" "MultiplyWithRoot" null null))
    (bind _projectilemovement (`/Game/FirstPerson/Blueprints/BP_FirstPersonProjectile.ProjectileMovement` _returnvalue))
    (bind _output_get (set `ProjectileMovementComponent.InitialSpeed` (`self.Bullet Speed`) _projectilemovement))
    (set `ProjectileMovementComponent.MaxSpeed` _output_get _projectilemovement)
    (set `self.LeftRailgun` false)
    (else
      (bind _returnvalue_2 (`|SpawnActorFromClass` "/Game/FirstPerson/Blueprints/BP_FirstPersonProjectile.BP_FirstPersonProjectile_C" (`SceneComponent.GetSocketTransform` (`self.StaticMesh`) "RightBarrel" "RTS_World") "Undefined" "MultiplyWithRoot" null null))
      (bind _projectilemovement_2 (`/Game/FirstPerson/Blueprints/BP_FirstPersonProjectile.ProjectileMovement` _returnvalue_2))
      (bind _output_get_2 (set `ProjectileMovementComponent.InitialSpeed` (`self.Bullet Speed`) _projectilemovement_2))
      (set `ProjectileMovementComponent.MaxSpeed` _output_get_2 _projectilemovement_2)
      (set `self.LeftRailgun` true))))

(fn `UserConstructionScript`)