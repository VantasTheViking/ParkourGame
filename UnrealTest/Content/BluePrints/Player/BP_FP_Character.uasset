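; First-person player character Blueprint that handles basic movement, look and jump through Enhanced Input.
; On BeginPlay it adds the IMC_DefaultTest mapping context to the owning player controller's input subsystem.
; Move input drives movement along the actor's right and forward vectors, look input feeds controller yaw and pitch, and jump input starts and stops jumping.
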(event `self.ReceiveBeginPlay`
  (bind _asplayer_controller (cast `PlayerController` (`self.GetController`)))
  (bind _returnvalue (pcsubsystem `EnhancedInputLocalPlayerSubsystem` _asplayer_controller))
  (`/Engine/EditorBlueprintResources/StandardMacros.IsValid` _returnvalue
    (:`Is Valid`
      (`EnhancedInputSubsystemInterface.AddMappingContext` _returnvalue "/Game/BluePrints/Player/InputActions/IMC_DefaultTest.IMC_DefaultTest" 0 (struct)))))

(event `EnhancedInput|/Game/BluePrints/Player/InputActions/IA_MoveTest`
  (params (ActionValue :type "Vector2D Structure") (ElapsedSeconds :type "Float (double-precision)") (TriggeredSeconds :type "Float (double-precision)") (InputAction :type "InputAction Object Reference" :default "/Game/BluePrints/Player/InputActions/IA_MoveTest.IA_MoveTest"))
  (bind (_x _y) (`KismetMathLibrary.BreakVector2D` ActionValue))
  (:`Triggered`
    (`self.AddMovementInput` (`self.GetActorRightVector`) _x)
    (`self.AddMovementInput` (`self.GetActorForwardVector`) _y)))

(event `EnhancedInput|/Game/BluePrints/Player/InputActions/IA_JumpTest`
  (params (ActionValue :type Boolean) (ElapsedSeconds :type "Float (double-precision)") (TriggeredSeconds :type "Float (double-precision)") (InputAction :type "InputAction Object Reference" :default "/Game/BluePrints/Player/InputActions/IA_JumpTest.IA_JumpTest"))
  (:`Triggered`
    (`self.Jump`))
  (:`Completed`
    (`self.StopJumping`)))

(event `EnhancedInput|/Game/BluePrints/Player/InputActions/IA_LookTest`
  (params (ActionValue :type "Vector2D Structure") (ElapsedSeconds :type "Float (double-precision)") (TriggeredSeconds :type "Float (double-precision)") (InputAction :type "InputAction Object Reference" :default "/Game/BluePrints/Player/InputActions/IA_LookTest.IA_LookTest"))
  (bind (_x _y) (`KismetMathLibrary.BreakVector2D` ActionValue))
  (:`Triggered`
    (`self.AddControllerYawInput` _x)
    (`self.AddControllerPitchInput` _y)))

(fn `UserConstructionScript`)