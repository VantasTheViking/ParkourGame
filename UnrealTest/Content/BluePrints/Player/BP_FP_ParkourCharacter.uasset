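; First-person parkour character Blueprint with Enhanced Input for moving, looking and jumping, plus early scaffolding for wall running.
; Move input feeds Gate-based walk, right wall-run and left wall-run states, with only walking applying movement so far.
; Each tick, sideways line traces from the capsule open the matching wall-run gate when a wall is hit while falling, otherwise closing it.
; Wall-climb detection is an empty stub.
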(event `self.ReceiveBeginPlay`
  (bind _asplayer_controller (cast `PlayerController` (`self.GetController`)))
  (bind _returnvalue (pcsubsystem `EnhancedInputLocalPlayerSubsystem` _asplayer_controller))
  (`/Engine/EditorBlueprintResources/StandardMacros.IsValid` _returnvalue
    (:`Is Valid`
      (`EnhancedInputSubsystemInterface.AddMappingContext` _returnvalue "/Game/BluePrints/Player/InputActions/IMC_DefaultParkour.IMC_DefaultParkour" 0 (struct)))))

(event `EnhancedInput|/Game/BluePrints/Player/InputActions/IA_MoveParkour`
  (params (ActionValue :type "Vector2D Structure") (ElapsedSeconds :type "Float (double-precision)") (TriggeredSeconds :type "Float (double-precision)") (InputAction :type "InputAction Object Reference" :default "/Game/BluePrints/Player/InputActions/IA_MoveParkour.IA_MoveParkour"))
  (:`Triggered`
    (`|ExecutionSequence`
      (:`then_0`
        (`self.WalkState` :!label _label))
      (:`then_1`
        (`self.RightWallRunState` :!label _label_2))
      (:`then_2`
        (`self.LeftWallRunState` :!label _label_3)))))

(event `OpenWalkGate`
  (goto _label :!via `Open`))

(event `CloseWalkGate`
  (goto _label :!via `Close`))

(event `OpenRightWallRunGate`
  (goto _label_2 :!via `Open`))

(event `CloseRightWallRunGate`
  (goto _label_2 :!via `Close`))

(event `OpenLeftWallRunGate`
  (goto _label_3 :!via `Open`))

(event `CloseLeftWallRunGAte`
  (goto _label_3 :!via `Close`))

(event `EnhancedInput|/Game/BluePrints/Player/InputActions/IA_JumpParkour`
  (params (ActionValue :type Boolean) (ElapsedSeconds :type "Float (double-precision)") (TriggeredSeconds :type "Float (double-precision)") (InputAction :type "InputAction Object Reference" :default "/Game/BluePrints/Player/InputActions/IA_JumpParkour.IA_JumpParkour"))
  (:`Triggered`
    (`self.Jump`))
  (:`Completed`
    (`self.StopJumping`)))

(event `EnhancedInput|/Game/BluePrints/Player/InputActions/IA_LookParkour`
  (params (ActionValue :type "Vector2D Structure") (ElapsedSeconds :type "Float (double-precision)") (TriggeredSeconds :type "Float (double-precision)") (InputAction :type "InputAction Object Reference" :default "/Game/BluePrints/Player/InputActions/IA_LookParkour.IA_LookParkour"))
  (bind (_x _y) (`KismetMathLibrary.BreakVector2D` (0.0 0.0)))
  (:`Triggered`
    (`self.AddControllerYawInput` _x)
    (`self.AddControllerPitchInput` _y)))

(event `self.ReceiveTick`
  (params (DeltaSeconds :type "Float (single-precision)"))
  (`|ExecutionSequence`
    (:`then_0`
      (`self.DetectRightWallRun`))
    (:`then_1`
      (`self.DetectLeftWallRun`))
    (:`then_2`
      (`self.DetectWallClimb`))))

(fn `DetectLeftWallRun`
  (bind _capsulecomponent (`self.CapsuleComponent`))
  (bind _returnvalue (`SceneComponent.K2_GetComponentLocation` _capsulecomponent))
  (bind (_outhit _returnvalue_2) (`KismetSystemLibrary.LineTraceSingle` :`Start` _returnvalue :`End` (+ _returnvalue (* (`SceneComponent.GetRightVector` _capsulecomponent) (* (`self.WallDetectionionRange`) -1.0))) :`TraceChannel` "TraceTypeQuery1" :`DrawDebugType` "ForOneFrame"))
  (if _returnvalue_2
    (if (`NavMovementComponent.IsFalling` (`self.CharacterMovement`))
      (`self.OpenLeftWallRunGate`)
      (else
        (`self.CloseLeftWallRunGAte` :!label _label)))
    (else
      (goto _label))))

(fn `DetectRightWallRun`
  (bind _capsulecomponent (`self.CapsuleComponent`))
  (bind _returnvalue (`SceneComponent.K2_GetComponentLocation` _capsulecomponent))
  (bind (_outhit _returnvalue_2) (`KismetSystemLibrary.LineTraceSingle` :`Start` _returnvalue :`End` (+ _returnvalue (* (`SceneComponent.GetRightVector` _capsulecomponent) (`self.WallDetectionionRange`))) :`TraceChannel` "TraceTypeQuery1" :`DrawDebugType` "ForOneFrame"))
  (if _returnvalue_2
    (if (`NavMovementComponent.IsFalling` (`self.CharacterMovement`))
      (`self.OpenRightWallRunGate`)
      (else
        (`self.CloseRightWallRunGate` :!label _label)))
    (else
      (goto _label))))

(fn `DetectWallClimb`)

(fn `UserConstructionScript`)