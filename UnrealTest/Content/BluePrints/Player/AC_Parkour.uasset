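; Parkour actor component that gives the player character wall running, wall jumping and camera roll, with wall climbing only stubbed.
; A looping timer traces left and right for suitably angled walls while falling, toggling per-side gates.
; On Tick, open gates launch the character along the wall using the normal-up cross product, and control rotation eases into a tilt.
; Jump launches off the wall and starts a cooldown that pauses wall-run movement.
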(event `Start`
  (params (Character :type "/Game/BluePrints/Player/BP_FP_ParkourCharacter Object Reference"))
  (`|ExecutionSequence`
    (:`then_0`
      (bind _output_get (set `self.PlayerCharacter` Character))
      (set `self.Character Movement` (`Character.CharacterMovement` _output_get)))
    (:`then_1`
      (`KismetSystemLibrary.K2_SetTimerDelegate` (delegate `WallRunUpdateEvent`) 0.1 true)
      (`KismetSystemLibrary.K2_SetTimerDelegate` (delegate `WallClimbUpdateEvent`) 0.1 true))))

(event `WallRunUpdateEvent`
  (`self.WallRunUpdate`))

(event `WallClimbUpdateEvent`
  (`self.WallClimbUpdate`))

(event `self.ReceiveTick`
  (params (DeltaSeconds :type "Float (single-precision)"))
  (`|ExecutionSequence`
    (:`then_0`
      (`/Engine/EditorBlueprintResources/StandardMacros.Gate` true :!label _label
        (:`Exit`
          (`self.LeftWallRun`))))
    (:`then_1`
      (`/Engine/EditorBlueprintResources/StandardMacros.Gate` true :!label _label_2
        (:`Exit`
          (`self.RightWallRun`))))
    (:`then_2`
      (`/Engine/EditorBlueprintResources/StandardMacros.Gate` true :!label _label_3))
    (:`then_3`
      (`self.CameraUpdate`))))

(event `OpenLeftWallRunGate`
  (goto _label :!via `Open`))

(event `CloseLeftWallRunGate`
  (goto _label :!via `Close`))

(event `OpenRightWallRunGate`
  (goto _label_2 :!via `Open`))

(event `CloseRightWallRunGate`
  (goto _label_2 :!via `Close`))

(event `OpenWallClimbGate`
  (goto _label_3 :!via `Open`))

(event `CloseWallClimbGate`
  (goto _label_3 :!via `Close`))

(event `Jump`
  (`self.WallJump`))

(event `ResetWallRunCooldown`
  (set `self.WallRunOnCooldown` false))

(event `StartWallRunCooldown`
  (set `self.WallRunOnCooldown` true)
  (`KismetSystemLibrary.K2_SetTimerDelegate` (delegate `ResetWallRunCooldown`) (`self.WallRunCooldownTime`)))

(fn `CameraUpdate`
  (locals (RWallTilt :type "Float (double-precision)" :default -35.0))
  (if (`self.IsWallRunningR`)
    (`self.CameraTilt` -15.0)
    (elif (`self.IsWallRunningL`)
      (`self.CameraTilt` 15.0)
      (else
        (`self.CameraTilt` 0.0)))))

(fn `LeftWallRun`
  (if (not (`self.WallRunOnCooldown`))
    (`Character.LaunchCharacter` (`self.PlayerCharacter`) (`self.WallMagnetism`) false false)
    (`Character.LaunchCharacter` (`self.PlayerCharacter`) (+ (* (`KismetMathLibrary.Cross_VectorVector` (`self.CurrentWallNormal`) (0.0 0.0 1.0)) (* (`self.WallRunSpeed`) 1.0)) (`KismetMathLibrary.MakeVector` 0.0 0.0 (* (`self.WallRunGravity`) -1.0))) true true)))

(fn `RightWallRun`
  (if (not (`self.WallRunOnCooldown`))
    (`Character.LaunchCharacter` (`self.PlayerCharacter`) (`self.WallMagnetism`) false false)
    (`Character.LaunchCharacter` (`self.PlayerCharacter`) (+ (* (`KismetMathLibrary.Cross_VectorVector` (`self.CurrentWallNormal`) (0.0 0.0 1.0)) (* (`self.WallRunSpeed`) -1.0)) (`KismetMathLibrary.MakeVector` 0.0 0.0 (* (`self.WallRunGravity`) -1.0))) true true)))

(fn `WallClimbUpdate`)

(fn `WallJump`
  (bind (_currentwallnormal_x _currentwallnormal_y) (`KismetMathLibrary.BreakVector` (`self.CurrentWallNormal`)))
  (bind _walljumphorizontalstrenght (`self.WallJumpHorizontalStrenght`))
  (if (`self.IsWallRunningR`)
    (`self.StartWallRunCooldown` :!label _label)
    (`Character.LaunchCharacter` (`self.PlayerCharacter`) (`KismetMathLibrary.MakeVector` (* _currentwallnormal_x _walljumphorizontalstrenght) (* _currentwallnormal_y _walljumphorizontalstrenght) (`self.WallJumpVerticalStrength`)) false true)
    (elif (`self.IsWallRunningL`)
      (goto _label))))

(fn `WallRunCooldown`
  (set `self.WallRunOnCooldown` true)
  (`KismetSystemLibrary.K2_SetTimerDelegate` _))

(fn `WallRunUpdate`
  (`|ExecutionSequence`
    (:`then_0`
      (`self.CheckLeftWallRun`))
    (:`then_1`
      (`self.CheckRightWallRun`))))